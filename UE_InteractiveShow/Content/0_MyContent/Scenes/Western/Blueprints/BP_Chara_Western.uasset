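; Western scene character Blueprint whose ActorTipe sets its role; construction shows the badge only for the sheriff and toggles the mask via LlevarMascara.
; MoveToDest triggers a walk animation and Timeline lerp to the destination, then notifies Manager; the Time input is ignored because SetPlayRate is unconnected.
; FSetAnimation plays an enum-selected animation directly on the mesh, returning its length.
; Click input only prints debug text, with an extra message for the sheriff.
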(event `Go-to`
  (params (Dest :type "Vector Structure") (Time :type "Float (double-precision)"))
  ; Goto with timeline
  (bind _output_get (set `self.StartLoc` (`self.K2_GetActorLocation`)))
  (`self.F_SetAnimation` "NewEnumerator7")
  (bind (_direction _alphamask) (`Timeline|Timeline` :!via `PlayFromStart`)
    (:`Update`
      (`self.K2_SetActorLocation` (`KismetMathLibrary.VLerp` _output_get Dest _alphamask)))
    (:`Finished`
      (`/Game/0_MyContent/Scenes/Western/Blueprints/BP_WesternManager.DestReached` (`self.Manager`)))))

(event `EnhancedInput|/Game/0_MyContent/Blueprints/IA_Click`
  (params (ActionValue :type Boolean) (ElapsedSeconds :type "Float (double-precision)") (TriggeredSeconds :type "Float (double-precision)") (InputAction :type "InputAction Object Reference" :default "/Game/0_MyContent/Blueprints/IA_Click.IA_Click"))
  (:`Started`
    (`KismetSystemLibrary.PrintString` "Clicked!")
    (switch `/Game/0_MyContent/Scenes/Western/Blueprints/DATA/E_WesternActors` (`self.ActorTipe`)
      (:`NewEnumerator3`
        (`KismetSystemLibrary.PrintString` "Soy el sherif -> ¿deberia disparar al hacer click?" true true (struct :`R` 1.0 :`G` 0.845891 :`B` 0.000508 :`A` 1.0))))))

(fn `F_SetAnimation`
  (params (Animation :type "/Game/0_MyContent/Scenes/Western/Blueprints/DATA/E_WesternAnimations Enum" :default "NewEnumerator4"))
  (returns (AnimationLenght :type "Float (double-precision)"))
  (bind _returnvalue (select `/Game/0_MyContent/Scenes/Western/Blueprints/DATA/E_WesternAnimations` Animation :`NewEnumerator4` "/Game/Prototyping/Characters/Mannequins/Anims/Unarmed/MM_Idle.MM_Idle" :`NewEnumerator7` "/Game/Prototyping/Characters/Mannequins/Anims/Unarmed/Walk/MF_Unarmed_Walk_Fwd.MF_Unarmed_Walk_Fwd" :`NewEnumerator3` "/Game/Prototyping/Characters/Mannequins/Anims/Pistol/MM_Pistol_Equip.MM_Pistol_Equip" :`NewEnumerator12` "/Game/Prototyping/Characters/Mannequins/Anims/Pistol/MF_Pistol_Idle_ADS.MF_Pistol_Idle_ADS" :`NewEnumerator13` "/Game/Prototyping/Characters/Mannequins/Anims/Pistol/Walk/MF_Pistol_Walk_Fwd.MF_Pistol_Walk_Fwd" :`NewEnumerator8` (`self.ShootAnim`) :`NewEnumerator11` "/Game/Prototyping/Characters/Mannequins/Anims/Pistol/MM_Pistol_Equip.MM_Pistol_Equip" :`NewEnumerator9` (`self.DeathAnim`)))
  ; Set custom animation
  (`SkeletalMeshComponent.PlayAnimation` (`self.Mesh`) _returnvalue (select `/Game/0_MyContent/Scenes/Western/Blueprints/DATA/E_WesternAnimations` Animation :`NewEnumerator4` true :`NewEnumerator7` true :`NewEnumerator12` true :`NewEnumerator13` true))
  (return (`AnimationAsset.GetPlayLength` _returnvalue)))

(fn `MoveToDest`
  (params (Dest :type "Vector Structure") (Time :type "Float (double-precision)"))
  (`self.Go-to` Dest Time)
  (return))

(fn `UserConstructionScript`
  (locals (NewLocalVar :type "SkeletalMeshComponent Object Reference"))
  (`|ExecutionSequence`
    (:`then_1`
      (`SceneComponent.SetVisibility` (`self.Placa`) (select `/Game/0_MyContent/Scenes/Western/Blueprints/DATA/E_WesternActors` (`self.ActorTipe`) :`NewEnumerator3` true) false))
    (:`then_2`
      (`SceneComponent.SetVisibility` (`self.Mask`) (`self.LlevarMascara`) false))))