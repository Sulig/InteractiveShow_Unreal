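; Manager for the Western scene's click-driven minigames, picking Duelo or Disparar from the show manager's channel and configuring light, hidden actors and camera.
; The duel walks sheriff and rival into place, cycles cameras randomly, then times a difficulty-scaled "DISPARA!" signal against the rival's shot.
; A gated click decides victory, defeat, draw or too early, plays animations and reports reaction times to the show manager.
; Disparar only has its setup and caption so far.
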(event `self.ReceiveBeginPlay`
  ;[0.04979 0.15 0.02427 0.5] Lights - Camera - ACTION!
  (`self.EnableInput` (`GameplayStatics.GetPlayerController` 0))
  (`self.SeleccionarMinijuego`))

(event `EnhancedInput|/Game/0_MyContent/Blueprints/Inputs/IA_Click`
  (params (ActionValue :type Boolean) (ElapsedSeconds :type "Float (double-precision)") (TriggeredSeconds :type "Float (double-precision)") (InputAction :type "InputAction Object Reference" :default "/Game/0_MyContent/Blueprints/Inputs/IA_Click.IA_Click"))
  ;[0 1 0.3487] Como la mecanica principal es hacer click en el lugar correcto o en cualquier lugar (dependiendo de la mini-escena), tendre que saber que evento cargar cuando se hace click.
  (:`Triggered`
    (`KismetSystemLibrary.PrintString` "Hello")
    (if ActionValue
      (switch `/Game/0_MyContent/Blueprints/DATA/E_Channels` (`self.MinigameName`)
        (:`NewEnumerator0`
          (`self.ClickerDuelo`))))))

(event `SeleccionarMinijuego`
  ; Externamente le pasare que minijuego quiero cargar, y dependiendo de cual, preparo una escena u otra y hago las condiciones + cinematicas
  (bind _channel (`/Game/0_MyContent/Blueprints/Mechanics/BPC_ShowManager.GetChannel` (`self.BPC_ShowManager`)))
  (bind _output_get (set `self.MinigameName` _channel))
  (switch `/Game/0_MyContent/Blueprints/DATA/E_Channels` _output_get
    (:`NewEnumerator0`
      (`self.StartDuelo`))
    (:`NewEnumerator1`
      (`self.StartDisparos`))))

(event `FinishScene`
  (params (WaitTime :type "Float (double-precision)" :default 1.0))
  ;[1 0.3816 0] Finish
  (`KismetSystemLibrary.K2_SetTimerDelegate` (select `/Game/0_MyContent/Blueprints/DATA/E_Channels` (`self.MinigameName`) :`NewEnumerator0` (delegate `FinishDuelo`)) WaitTime))

(event `FinishDuelo`
  ;[1 0.3816 0] Finish
  (`self.F_FinishDuelo`))

(event `DCargarAnimacionesConjuntas`
  (params (Animacion :type "/Game/0_MyContent/Scenes/Western/Blueprints/DATA/E_WesternAnimations Enum" :default "NewEnumerator4"))
  ;[0 0.15 0.1212 0.5] Esto es SOLO para cargar animaciones conjuntas para los dos actores
  (`|ExecutionSequence`
    (:`then_0`
      (`/Game/0_MyContent/Scenes/Western/Blueprints/BP_Chara_Western.F_SetAnimation` (`self.DSherif`) Animacion false))
    (:`then_1`
      (`/Game/0_MyContent/Scenes/Western/Blueprints/BP_Chara_Western.F_SetAnimation` (`self.DRival`) Animacion false))))

(event `CallChangeCameraAgain`
  ;[0 0.15 0.1212 0.5] Cambio de camaras
  (bind _output_get (set `self.DChangeCmTimer` (`KismetMathLibrary.RandomFloatInRange` (`self.DMinCangeCamTime`) (`self.DMaxCangeCamTime`))))
  (`self.DChangeCameraWithTimer` null (`self.CamChangeRepitingTimesLeft`) _output_get))

(event `ClickerDuelo`
  (bind _rivalreactiontime (`self.RivalReactionTime`))
  (bind _playerreactiontime (`self.PlayerReactionTime`))
  ;[1 0 0.05823] Clicker
  (set `self.PlayerReactionTime` (- (`KismetSystemLibrary.GetGameTimeInSeconds`) (`self.ReactionStartTime`)))
  (`/Engine/EditorBlueprintResources/StandardMacros.Gate` true :!label _label
    (:`Exit`
      (switch `/Game/0_MyContent/Scenes/Western/Blueprints/DATA/E_WesternDueloStates` (`self.DueloState`)
        (:`NewEnumerator1`
          (`self.LoadSceneFinish` "NewEnumerator9"))
        (:`NewEnumerator2`
          (`KismetSystemLibrary.PrintString` (`KismetStringLibrary.Concat_StrStr` "He disparado en el tiempo justo -> mirame los tiempos!" " - my time: " (`KismetStringLibrary.Conv_DoubleToString` (`self.PlayerReactionTime`)) " - Enemy time - " (`KismetStringLibrary.Conv_DoubleToString` (`self.RivalReactionTime`))))
          (if (!= _rivalreactiontime 0.0)
            (if (< _playerreactiontime _rivalreactiontime)
              (`self.LoadSceneFinish` "NewEnumerator0" :!label _label_2)
              (`self.CloseCanShootGate`)
              (elif (== _playerreactiontime _rivalreactiontime)
                (`self.LoadSceneFinish` "NewEnumerator2")
                (`self.CloseCanShootGate`)
                (else
                  (`self.LoadSceneFinish` "NewEnumerator1")
                  (`self.CloseCanShootGate`))))
            (else
              (`KismetSystemLibrary.PrintString` "Eso es que el jugador ha disparado incluso antes que el enemigo - ¿no?")
              (goto _label_2))))
        (:`NewEnumerator3`
          (`self.LoadSceneFinish` "NewEnumerator10"))))))

(event `OpenCanShootGate`
  ;[1 0 0.05823] Clicker
  (goto _label :!via `Open`))

(event `/Game/0_MyContent/Scenes/Western/Blueprints/BPI_ActorsManager.DestReached`
  ;[0.04979 0.15 0.02427 0.5] Los actores han llegado a su destino -> ahora deberian prepararse para disparar
  (bind _result (`/Engine/EditorBlueprintResources/StandardMacros.IncrementInt` (`self.DReadyCharas`))
    (:`  `
      (if (>= _result 2)
        (`self.DCargarAnimacionesConjuntas` "NewEnumerator4")
        (`self.Desenfundar&Disparar`)))))

(event `CloseCanShootGate`
  ;[1 0 0.05823] Clicker
  (goto _label :!via `Close`))

(event `StartDuelo`
  ;[0.03958 1 0] Start duelo -> los dos empiezan a caminar
  (`self.PrepararEscena` "NewEnumerator0")
  (set `self.DueloState` "NewEnumerator0")
  (set `self.DCamTargets_cpy` (`self.DCamTargets`))
  (`|ExecutionSequence`
    (:`then_0`
      ;;[1 1 0.000508 0.5391] Esto setea (mediante un timer) cuanto tiempo esperará en contrincante en disparar (como veis, sera random y se puede modificar segun la dificultad)
      (bind _difficulty (`/Game/0_MyContent/Blueprints/Mechanics/BPC_ShowManager.GetDifficulty` (`self.BPC_ShowManager`)))
      (`|ExecutionSequence`
        (:`then_0`
          (set `self.RivalReactionTime` (select `int` _difficulty :`0` (`KismetMathLibrary.RandomFloatInRange` 0.6 1.0) :`1` (`KismetMathLibrary.RandomFloatInRange` 0.1 0.8))))
        (:`then_1`
          (set `self.ReactionStartTime` (select `int` _difficulty :`0` (`KismetMathLibrary.RandomFloatInRange` 1.8 2.2) :`1` (`KismetMathLibrary.RandomFloatInRange` 1.5 2.0))))))
    (:`then_1`
      (`/Game/0_MyContent/Scenes/Western/Blueprints/BPI_ActorsManager.MoveToDest` (`self.DRival`) (`SceneComponent.RelativeLocation` (`self.Duelo_ElMaloWalkTo`)) 0.0 self))
    (:`then_2`
      (`/Game/0_MyContent/Scenes/Western/Blueprints/BPI_ActorsManager.MoveToDest` (`self.DSherif`) (`SceneComponent.RelativeLocation` (`self.Duelo_SherifWalkTo`)) 0.0 self))
    (:`then_3`
      (`self.DChangeCameraWithTimer` (`self.DInitialCam`) (`self.CamChangeRepitingTimes`) (`KismetMathLibrary.RandomFloatInRange` (`self.DMinCangeCamTime`) (`self.DMaxCangeCamTime`))))))

(event `Desenfundar&Disparar`
  ;[1 1 0.000508 0.5391] Controlar tiempos de disparo
  (`|ExecutionSequence`
    (:`then_0`
      (set `self.DueloState` "NewEnumerator1")
      (`self.OpenCanShootGate`))
    (:`then_1`
      (`/Game/0_MyContent/Blueprints/UI/WBP_ActionCaption.ChangeCaptionActionText` (`/Game/0_MyContent/Blueprints/Mechanics/BP_PlayerControler_Show.Caption_HUD` (`/Game/0_MyContent/Blueprints/Mechanics/BPC_ShowManager.PlayerCntrShow` (`self.BPC_ShowManager`))) "Preparaos..")
      (`self.DCargarAnimacionesConjuntas` "NewEnumerator3")
      (`KismetSystemLibrary.K2_SetTimerDelegate` (delegate `EV_CanShoot`) (`self.ReactionStartTime`)) ; Espera un tiempo x- random antes de que aparezca 'dispara' - > esto se podra modificar segun la dificultad para que apareza antes o despues
    )))

(event `EV_CanShoot`
  ;[1 1 0.000508 0.5391] Controlar tiempos de disparo
  (`self.DCargarAnimacionesConjuntas` "NewEnumerator12")
  (`|ExecutionSequence`
    (:`then_0`
      (`/Game/0_MyContent/Blueprints/UI/WBP_ActionCaption.ChangeCaptionActionText` (`/Game/0_MyContent/Blueprints/Mechanics/BP_PlayerControler_Show.Caption_HUD` (`/Game/0_MyContent/Blueprints/Mechanics/BPC_ShowManager.PlayerCntrShow` (`self.BPC_ShowManager`))) "DISPARA!"))
    (:`then_1`
      (set `self.DueloState` "NewEnumerator2"))
    (:`then_2`
      (set `self.ReactionStartTime` (`KismetSystemLibrary.GetGameTimeInSeconds`))
      (bind _returnvalue (`KismetSystemLibrary.K2_SetTimerDelegate` (delegate `ThiefShoot`) (`self.RivalReactionTime`)))
      (set `self.RivalTimer` _returnvalue))))

(event `ThiefShoot`
  (bind _drival (`self.DRival`))
  ;[1 1 0.000508 0.5391] Controlar tiempos de disparo
  (switch `/Game/0_MyContent/Scenes/Western/Blueprints/DATA/E_WesternDueloStates` (`self.DueloState`)
    (:`NewEnumerator2`
      (`|ExecutionSequence`
        (:`then_0`
          (`self.CloseCanShootGate`)
          (`self.LoadSceneFinish` "NewEnumerator1"))
        (:`then_1`
          (bind _animationlenght (`/Game/0_MyContent/Scenes/Western/Blueprints/BP_Chara_Western.F_SetAnimation` _drival "NewEnumerator8" false))
          (`KismetSystemLibrary.Delay` _animationlenght)
          (`/Game/0_MyContent/Scenes/Western/Blueprints/BP_Chara_Western.F_SetAnimation` _drival "NewEnumerator12" false))))))

(event `LoadSceneFinish`
  (params (DueloResult :type "/Game/0_MyContent/Blueprints/DATA/E_SceneResult Enum" :default "NewEnumerator9"))
  ;[0 1 0.3487] Animaciones de morir / ganar - Segun lo que haya pasado
  (`|ExecutionSequence`
    (:`then_0`
      (set `self.DueloState` "NewEnumerator3"))
    (:`then_1`
      (`KismetSystemLibrary.K2_ClearAndInvalidateTimerHandle` (`self.ChangeCamTH`))
      (`KismetSystemLibrary.K2_ClearAndInvalidateTimerHandle` (`self.RivalTimer`)))
    (:`then_2`
      (bind _output_get (set `self.Duelo Result` DueloResult))
      (switch `/Game/0_MyContent/Blueprints/DATA/E_SceneResult` _output_get
        (:`NewEnumerator9`
          (`KismetSystemLibrary.PrintString` "Has disparado muy pronto")
          (`self.FinishScene` 1.0))
        (:`NewEnumerator2`
          (`KismetSystemLibrary.PrintString` "Empate --" true true (struct :`R` 0.221991 :`B` 1.0 :`A` 1.0))
          (`|ExecutionSequence`
            (:`then_0`
              (`/Game/0_MyContent/Scenes/Western/Blueprints/BP_Chara_Western.F_SetAnimation` (`self.DSherif`) "NewEnumerator9" false))
            (:`then_1`
              (`/Game/0_MyContent/Scenes/Western/Blueprints/BP_Chara_Western.F_SetAnimation` (`self.DRival`) "NewEnumerator9" false))
            (:`then_2`
              (`self.FinishScene` (`self.WaitTime_BeforeFinishDuelo`)))))
        (:`NewEnumerator1`
          (`KismetSystemLibrary.PrintString` "El Contrincante gana" true true (struct :`R` 1.0 :`A` 1.0))
          (`|ExecutionSequence`
            (:`then_0`
              (`self.DChangeCameraWithTimer` (`self.DRival`)))
            (:`then_1`
              (`/Game/0_MyContent/Scenes/Western/Blueprints/BP_Chara_Western.F_SetAnimation` (`self.DRival`) "NewEnumerator11" false))
            (:`then_2`
              (`/Game/0_MyContent/Scenes/Western/Blueprints/BP_Chara_Western.F_SetAnimation` (`self.DSherif`) "NewEnumerator9" false))
            (:`then_3`
              (`self.FinishScene` (`self.WaitTime_BeforeFinishDuelo`)))))
        (:`NewEnumerator0`
          (`KismetSystemLibrary.PrintString` "El Sherif gana" true true (struct :`R` 0.039578 :`G` 1.0 :`A` 1.0))
          (`|ExecutionSequence`
            (:`then_0`
              (`self.DChangeCameraWithTimer` (`self.DSherif`)))
            (:`then_1`
              (bind _animationlenght (`/Game/0_MyContent/Scenes/Western/Blueprints/BP_Chara_Western.F_SetAnimation` (`self.DSherif`) "NewEnumerator8" false))
              (`KismetSystemLibrary.Delay` _animationlenght)
              (`|ExecutionSequence`
                (:`then_0`
                  (`/Game/0_MyContent/Scenes/Western/Blueprints/BP_Chara_Western.F_SetAnimation` (`self.DRival`) "NewEnumerator9" false))
                (:`then_1`
                  (`/Game/0_MyContent/Scenes/Western/Blueprints/BP_Chara_Western.F_SetAnimation` (`self.DSherif`) "NewEnumerator11" false))
                (:`then_2`
                  (`self.FinishScene` (`self.WaitTime_BeforeFinishDuelo`)))))))))))

(event `StartDisparos`
  (`self.PrepararEscena` "NewEnumerator1")
  (`|ExecutionSequence`
    (:`then_0`
      (`/Game/0_MyContent/Blueprints/Mechanics/BPC_ShowManager.GetDifficulty` (`self.BPC_ShowManager`)))
    (:`then_1`
      (`/Game/0_MyContent/Blueprints/UI/WBP_ActionCaption.ChangeCaptionActionText` (`/Game/0_MyContent/Blueprints/Mechanics/BP_PlayerControler_Show.Caption_HUD` (`/Game/0_MyContent/Blueprints/Mechanics/BPC_ShowManager.PlayerCntrShow` (`self.BPC_ShowManager`))) "DISPARA!"))))

(fn `DChangeCameraWithTimer`
  (params (FirstObjective :type "Actor Object Reference") (RepitingTimes :type Integer :default 1) (Timer :type "Float (double-precision)"))
  (locals (LastObjective :type "Actor Object Reference"))
  (bind _dcamtargets_cpy (`self.DCamTargets_cpy`))
  (bind _dcamtargets_cpy_2 (`self.DCamTargets_cpy`))
  (bind _result (`/Engine/EditorBlueprintResources/StandardMacros.DecrementInt` RepitingTimes)
    (:`  `
      (bind _output_get (set `self.CamChangeRepitingTimesLeft` _result))
      (`|ExecutionSequence`
        (:`then_0`
          (if (== (`KismetArrayLibrary.Array_Length` _dcamtargets_cpy_2) 0)
            (set `self.DCamTargets_cpy` (`self.DCamTargets`))))
        (:`then_1`
          (bind _output_get_2 (set `self.DCamActualTarget` (select `bool` (`KismetSystemLibrary.IsValid` FirstObjective) :`false` (`KismetArrayLibrary.Array_Random` _dcamtargets_cpy_2) :`true` FirstObjective)))
          (`|ExecutionSequence`
            (:`then_0`
              (`PlayerController.SetViewTargetWithBlend` (`GameplayStatics.GetPlayerController` 0) _output_get_2 0.25 "VTBlend_EaseInOut" 0.0 false)
              (if (> _output_get 0)
                (if (> Timer 0.0)
                  (bind _returnvalue (`KismetSystemLibrary.K2_SetTimerDelegate` (`|CreateDelegate` :!event `CallChangeCameraAgain`) Timer))
                  (set `self.ChangeCamTH` _returnvalue))))
            (:`then_1`
              (if (!= (`KismetArrayLibrary.Array_Length` _dcamtargets_cpy) 0)
                (`KismetArrayLibrary.Array_RemoveItem` _dcamtargets_cpy (`self.DCamActualTarget`))
                (else
                  (set `self.DCamTargets_cpy` (`self.DCamTargets`)))))))))))

(fn `F_FinishDuelo`
  (bind _duelo_result (`self.Duelo Result`))
  (`/Game/0_MyContent/Blueprints/Mechanics/BPC_ShowManager.FinishScene` (`self.BPC_ShowManager`) (make `/Game/0_MyContent/Blueprints/DATA/S_SceneResult` :`MicroSceneID` (`self.MinigameName`) :`Result` (`self.Duelo Result`) :`Performance` (make `/Game/0_MyContent/Blueprints/DATA/S_PerformanceData` :`YourReactionTime` (`self.PlayerReactionTime`) :`EnemyReactionTime` (`self.RivalReactionTime`) :`ObjectsHit` (select `/Game/0_MyContent/Blueprints/DATA/E_SceneResult` _duelo_result :`NewEnumerator2` 1 :`NewEnumerator0` 1) :`ObjectsMissed` (select `/Game/0_MyContent/Blueprints/DATA/E_SceneResult` _duelo_result :`NewEnumerator6` 1 :`NewEnumerator10` 1 :`NewEnumerator9` 1 :`NewEnumerator1` 1 :`NewEnumerator7` 1)))))

(fn `PrepararEscena`
  (params (Escena :type "/Game/0_MyContent/Blueprints/DATA/E_Channels Enum" :default "NewEnumerator0"))
  (switch `/Game/0_MyContent/Blueprints/DATA/E_Channels` Escena
    (:`NewEnumerator0`
      ; Duelo config
      (`|ExecutionSequence`
        (:`then_0`
          (`self.K2_SetActorRotation` (`self.DSunLight`) (struct :`Pitch` -7.0 :`Yaw` 100.0) false))
        (:`then_1`
          (for _array_element (`self.HiddenDueloActors`)
            (`self.SetActorHiddenInGame` _array_element true)))
        (:`then_2`
          (`PlayerController.SetViewTargetWithBlend` (`GameplayStatics.GetPlayerController` 0) (`self.DInitialCam`) 0.0 "VTBlend_Linear" 0.0 false))
        (:`then_3`
          (`self.DCargarAnimacionesConjuntas` "NewEnumerator4"))))
    (:`NewEnumerator1`
      ; Dispararo al objetivo (version con bandidos) - config
      (`|ExecutionSequence`
        (:`then_0`
          (`self.K2_SetActorRotation` (`self.DSunLight`) (struct :`Pitch` -7.0 :`Yaw` 100.0) false))
        (:`then_1`
          (for _array_element_2 (`self.HiddenShootActors`)
            (`self.SetActorHiddenInGame` _array_element_2 true)))
        (:`then_2`
          (`PlayerController.SetViewTargetWithBlend` (`GameplayStatics.GetPlayerController` 0) (`self.SInitialCam`) 0.0 "VTBlend_Linear" 0.0 false))))))

(fn `UserConstructionScript`)