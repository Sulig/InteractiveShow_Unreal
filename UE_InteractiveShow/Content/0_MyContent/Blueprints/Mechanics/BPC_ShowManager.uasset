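; BPC_ShowManager is a component that manages show state: the current, next and last channel, the difficulty, and the end of a scene.
; Channel and difficulty accessors read and write GI_Show, the game instance, so state can carry across levels.
; FinishScene stores the result, runs PerformanceCalculator and opens the host level.
; Scoring is unfinished: partial score terms are computed but never saved to the game instance, and FinalScore is empty.
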(event `self.ReceiveBeginPlay`
  (`|ExecutionSequence`
    (:`then_0`
      (bind (_ok _gameinstance) (`self.GetGameInstance`))
      (if _ok
        (set `self.GI_Show` _gameinstance)))
    (:`then_1`
      (bind _asbp_player_controler_show (cast `/Game/0_MyContent/Blueprints/Mechanics/BP_PlayerControler_Show` (`GameplayStatics.GetPlayerController` 0))
        (:`then`
          (set `self.PlayerCntrShow` _asbp_player_controler_show))
        (:`CastFailed`
          (`KismetSystemLibrary.PrintText` "Platyer cast failed"))))))

(fn `FinalScore`)

(fn `FinishScene`
  (params (SceneResult :type "/Game/0_MyContent/Blueprints/DATA/S_SceneResult Structure"))
  (set `self.S_SceneResult` SceneResult)
  (`self.PerformanceCalculator`)
  (`GameplayStatics.OpenLevel` (`self.HostScene`)))

(fn `GetChannel`
  (returns (Channel :type "/Game/0_MyContent/Blueprints/DATA/E_Channels Enum"))
  (bind (_ok _gameinstance) (`self.GetGameInstance`))
  (if _ok
    (bind _output_get (set `/Game/0_MyContent/Blueprints/GI_Show.CurrentChanel` (`/Game/0_MyContent/Blueprints/GI_Show.NextChanel` _gameinstance) _gameinstance))
    (return _output_get)
    (else
      (return "NewEnumerator3"))))

(fn `GetDifficulty`
  (returns (Difficulty :type Integer))
  (bind (_ok _gameinstance) (`self.GetGameInstance`))
  (if _ok
    (return (`/Game/0_MyContent/Blueprints/GI_Show.CurrentDificulty` _gameinstance))
    (else
      (return 0))))

(fn `GetGameInstance`
  (returns (OK :type Boolean) (GameInstance :type "/Game/0_MyContent/Blueprints/GI_Show Object Reference"))
  (bind _asgi_show (cast `/Game/0_MyContent/Blueprints/GI_Show` (`GameplayStatics.GetGameInstance`))
    (:`then`
      (bind _output_get (set `self.GI_Show` _asgi_show))
      (return true _output_get))
    (:`CastFailed`
      (`KismetSystemLibrary.PrintText` "Cast failed in getting GameInstance! Maybe you forget to set it in prokect settings?" true true (struct :`R` 1.0 :`G` 0.061463 :`A` 1.0))
      (return false null))))

(fn `PerformanceCalculator`
  (locals (SInitial :type Integer) (SDifficulty :type Integer :default 0) (SAcurancy :type Integer) (SReaction :type Integer))
  (bind ((`ObjectsHit_10_6506C48F4C1AC449D5BD36AC859691E1` _objectshit) (`ObjectsMissed_12_34E039FF4B75A4FC89B9CDA3A781D4C3` _objectsmissed) (`TotalObjectives_30_8A55615A48777D194438D0B597D74C5D` _totalobjectives)) (break `/Game/0_MyContent/Blueprints/DATA/S_PerformanceData` (`self.Performance`)))
  (bind ((`TimeRemaining_15_F99F42494C9525AC29C851BF8162D3D6` _timeremaining) (`YourReactionTime_27_FB62891049D640448175C6B0981D9E30` _yourreactiontime) (`EnemyReactionTime_26_077B64BB4DF4882E517F76BE4658C8A9` _enemyreactiontime)) (break `/Game/0_MyContent/Blueprints/DATA/S_PerformanceData` (`self.Performance`)))
  (`KismetSystemLibrary.PrintString` "Finished -> Esto deberia calcular la puntuacion dependiendo del resultado + luego pasarlo al gameinstance + luego hacer lo correspondiente en la escena del host")
  (set `self.Performance` (`.Performance_23_D98692024C72C8C3A32F88B849BBE68A` (break `/Game/0_MyContent/Blueprints/DATA/S_SceneResult` (`self.S_SceneResult`))))
  (`|ExecutionSequence`
    (:`then_0`
      (bind _difficulty (`self.GetDifficulty`))
      (set `local.SDifficulty` _difficulty))
    (:`then_1`
      (set `local.SInitial` (select `/Game/0_MyContent/Blueprints/DATA/E_SceneResult` (`.Result_5_B6FCBEEB4EFE4BAC599460A93E8CFFF1` (break `/Game/0_MyContent/Blueprints/DATA/S_SceneResult` (`self.S_SceneResult`))) :`NewEnumerator2` 25 :`NewEnumerator0` 50 :`NewEnumerator7` 10)))
    (:`then_2`
      (set `local.SAcurancy` (* (/ _objectshit _totalobjectives) 10))
      (setmembers `/Game/0_MyContent/Blueprints/DATA/S_PerformanceData` :`StructRef` (`self.Performance`) :`Accurancy` (/ _objectshit _totalobjectives)))
    (:`then_3`
      (if (< _yourreactiontime _enemyreactiontime)
        (set `local.SReaction` 0)))))

(fn `SetChannel`
  (params (Scene :type "/Game/0_MyContent/Blueprints/DATA/E_Channels Enum" :default "NewEnumerator3"))
  (returns (OK :type Boolean))
  (bind (_ok _gameinstance) (`self.GetGameInstance`))
  (if _ok
    (set `/Game/0_MyContent/Blueprints/GI_Show.LastChanel` (`/Game/0_MyContent/Blueprints/GI_Show.CurrentChanel` _gameinstance) _gameinstance)
    (set `/Game/0_MyContent/Blueprints/GI_Show.NextChanel` Scene _gameinstance)
    (return true)
    (else
      (return false))))

(fn `SetDifficulty`
  (params (Difficulty :type Integer))
  (returns (Ok :type Boolean))
  (bind (_ok _gameinstance) (`self.GetGameInstance`))
  (if _ok
    (set `/Game/0_MyContent/Blueprints/GI_Show.CurrentDificulty` Difficulty _gameinstance)
    (return true)
    (else
      (return false))))