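; Component meant to score performance when a show scene ends and return play to the host scene, with scoring still a stub.
; On BeginPlay it caches the show GameInstance and player controller.
; FinishScene calls the empty CalculatePerformance, leaving its channel and result inputs unused, then opens HostScene.
; SeleccionarMinijuego returns the next channel stored in the GameInstance, or a fixed default if that lookup fails.
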(event `self.ReceiveBeginPlay`
  (`|ExecutionSequence`
    (:`then_0`
      (bind (_ok _gameinstance) (`self.GetGameInstance`))
      (if _ok
        (set `self.GI_Show` _gameinstance)))
    (:`then_1`
      (bind _asbp_player_controler_show (cast `/Game/0_MyContent/Blueprints/Mechanics/BP_PlayerControler_Show` (`GameplayStatics.GetPlayerController` 0))
        (:`then`
          (set `self.PlayerCntrShow` _asbp_player_controler_show))
        (:`CastFailed`
          (`KismetSystemLibrary.PrintText` "Platyer cast failed"))))))

(fn `CalculatePerformance`)

(fn `FinishScene`
  (params (Channel :type "/Game/0_MyContent/Blueprints/DATA/E_Channels Enum" :default "NewEnumerator3") (SceneResult :type "/Game/0_MyContent/Blueprints/DATA/E_SceneResult Enum" :default "NewEnumerator6"))
  (`KismetSystemLibrary.PrintString` "Finished -> Esto deberia calcular la puntuacion dependiendo del resultado + luego pasarlo al gameinstance + luego hacer lo correspondiente en la escena del host")
  (`self.CalculatePerformance`)
  (`GameplayStatics.OpenLevel` (`self.HostScene`)))

(fn `GetGameInstance`
  (returns (OK :type Boolean) (GameInstance :type "/Game/0_MyContent/Blueprints/GI_Show Object Reference"))
  (bind _asgi_show (cast `/Game/0_MyContent/Blueprints/GI_Show` (`GameplayStatics.GetGameInstance`))
    (:`then`
      (bind _output_get (set `self.GI_Show` _asgi_show))
      (return true _output_get))
    (:`CastFailed`
      (`KismetSystemLibrary.PrintText` "Cast failed in getting GameInstance! Maybe you forget to set it in prokect settings?" true true (struct :`R` 1.0 :`G` 0.061463 :`A` 1.0))
      (return false null))))

(fn `SeleccionarMinijuego`
  (returns (Channel :type "/Game/0_MyContent/Blueprints/DATA/E_Channels Enum"))
  (bind (_ok _gameinstance) (`self.GetGameInstance`))
  (if _ok
    (return (`/Game/0_MyContent/Blueprints/GI_Show.NextChanel` _gameinstance))
    (else
      (return "NewEnumerator3"))))