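; BP_Subway is a metro train actor that moves itself to a stop and can later travel on to a final destination.
; BeginPlay waits a configurable delay, then sends the train to the stop; GoToFinal is a separate event with no caller in this graph.
; Both use a shared GoTo event, where a timeline alpha lerps the actor from its current location to the target without sweep.
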(event `GoToStopDest`
  ; GotoStop
  (`self.GoTo` (`self.StopDest`) 5.0))

(event `GoToFinal`
  ; GotoFinal
  (`self.GoTo` (`self.FinalDest`) 4.0))

(event `self.ReceiveBeginPlay`
  ;[0 0.4678 0.1421] Begin play - Colocar Subway in the start position and goto stop destination (parada de metro)
  (`KismetSystemLibrary.Delay` (`self.WaitTimeToStart`))
  (`self.GoToStopDest`))

(event `GoTo`
  (params (Destination :type "Vector Structure") (Lenght :type "Float (double-precision)"))
  ;[0.9688 0.9688 0.9688 0.5] Subway - Goto - Animation
  (bind _output_get (set `self.ActualLoc` (`self.K2_GetActorLocation`)))
  (bind (_direction _alphamask) (`Timeline|Timeline` :`NewTime` Lenght :!via `PlayFromStart`)
    (:`Update`
      (`self.K2_SetActorLocation` (`KismetMathLibrary.VLerp` _output_get Destination _alphamask)))))

(fn `UserConstructionScript`)